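; Switchable electric fence hazard that spans from the actor origin to an EndPoint, extending a parent switchable Blueprint.
; The construction script centers, aims and stretches an invisible HazardMesh along that span, moves the End component to EndPoint, and feeds the point to the particle system as EndPosition.
; Switch on and off events call the parent logic, then start or stop the particle effect and sound.
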(event `/Game/PGTemplate/Blueprints/Objects/Core/SwitchInterface.SwitchOn`
  (`parent.SwitchOn`)
  (`ActorComponent.Activate` (`self.ParticleSystem`) false)
  (`AudioComponent.Play` (`self.Sound`) 0.0))

(event `/Game/PGTemplate/Blueprints/Objects/Core/SwitchInterface.SwitchOff`
  (`parent.SwitchOff`)
  (`ActorComponent.Deactivate` (`self.ParticleSystem`))
  (`AudioComponent.Stop` (`self.Sound`)))

(fn `UserConstructionScript`
  (bind _endpoint (`self.EndPoint`))
  (bind _hazardmesh (`self.HazardMesh`))
  (`SceneComponent.K2_SetRelativeLocation` _hazardmesh (/ _endpoint 2.0) false false)
  (`SceneComponent.K2_SetRelativeRotation` _hazardmesh (`KismetMathLibrary.FindLookAtRotation` (0.0 0.0 0.0) _endpoint) false false)
  (`SceneComponent.SetRelativeScale3D` _hazardmesh (`KismetMathLibrary.MakeVector` (* (`KismetMathLibrary.VSize` _endpoint) 0.01) 0.6 0.1))
  (`SceneComponent.K2_SetRelativeLocation` (`self.End`) (`self.EndPoint`) false false)
  (`parent.UserConstructionScript`)
  (`SceneComponent.SetVisibility` (`self.HazardMesh`) false false)
  (`NiagaraComponent.SetVariableVec3` (`self.ParticleSystem`) "EndPosition" (`self.EndPoint`)))