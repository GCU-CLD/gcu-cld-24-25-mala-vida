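; SwitchableHazard_BP is a hazard object that can be switched on and off.
; Switching on enables HazardMesh query and physics collision and makes its material fully opaque, while switching off disables collision and fades the material through its Opacity parameter.
; Both events act only when the IsOn flag would change, and SetInitialStatus routes to one of them.
; GetStatus exposes IsOn to callers.
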(event `/Game/PGTemplate/Blueprints/Objects/Core/SwitchInterface.SwitchOn`
  (if (not (`self.isOn`))
    (set `self.isOn` true)
    (`PrimitiveComponent.SetCollisionEnabled` (`self.HazardMesh`) "QueryAndPhysics")
    (`MaterialInstanceDynamic.SetScalarParameterValue` (`self.Material`) "Opacity" 1.0)))

(event `/Game/PGTemplate/Blueprints/Objects/Core/SwitchInterface.SwitchOff`
  (if (`self.isOn`)
    (set `self.isOn` false)
    (`PrimitiveComponent.SetCollisionEnabled` (`self.HazardMesh`) "NoCollision")
    (`MaterialInstanceDynamic.SetScalarParameterValue` (`self.Material`) "Opacity" 0.2)))

(event `/Game/PGTemplate/Blueprints/Objects/Core/SwitchInterface.SetInitialStatus`
  (params (InitialStatus :type Boolean))
  (if InitialStatus
    (`self.SwitchOn`)
    (else
      (`self.SwitchOff`))))

(fn `GetStatus`
  (returns (isOn :type Boolean))
  (return (`self.isOn`)))

(fn `UserConstructionScript`
  (`parent.UserConstructionScript`))