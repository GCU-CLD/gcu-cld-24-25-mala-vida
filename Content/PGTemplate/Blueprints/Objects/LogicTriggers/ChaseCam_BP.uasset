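; Trigger actor for an auto-scrolling chase sequence: overlap shows a chase object and blends the player's view to a spline-following camera.
; A timeline paced by spline length and speed updates the camera and projects the chase object to a screen edge based on travel direction.
; Leaving the camera's FOV deals damage equal to the player's Health and restores the pawn view, as does finishing.
; OnReset re-arms the one-shot trigger.
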(event `self.TriggerBOx.OnComponentBeginOverlap`
  (params (OverlappedComponent :type "PrimitiveComponent Object Reference") (OtherActor :type "Actor Object Reference") (OtherComp :type "PrimitiveComponent Object Reference") (OtherBodyIndex :type Integer) (bFromSweep :type Boolean) (SweepResult :type "HitResult Structure (by ref)"))
  (bind _returnvalue (`GameplayStatics.GetPlayerController` 0))
  (bind _returnvalue_2 (`GameplayStatics.GetPlayerController` 0))
  (bind _returnvalue_3 (`Controller.K2_GetPawn` _returnvalue_2))
  (bind _asbp_player_character (cast `/Game/PGTemplate/Blueprints/Characters/Player/BP_PlayerCharacter` _returnvalue_3 :!pure true))
  (`/Engine/EditorBlueprintResources/StandardMacros.DoOnce` false :!label _label
    (:`Completed`
      (`SceneComponent.SetVisibility` (`self.ChaseObjectHandle`) true true)
      (cast `/Game/PGTemplate/Blueprints/Characters/Player/BP_PlayerCharacter` OtherActor)
      (`PlayerController.SetViewTargetWithBlend` (`GameplayStatics.GetPlayerController` 0) self (`self.TransitionInTime`) "VTBlend_Linear" 0.0 false)
      (`TimelineComponent.SetPlayRate` (`self.CameraMovementTimeline`) (/ 1.0 (/ (`SplineComponent.GetSplineLength` (`self.CameraMotionSpline`)) (`self.CameraMoveSpeedSteady`))))
      (`Timeline|CameraMovementTimeline` :!via `PlayFromStart` :!label _label_2
        (:`Update`
          (set `self.TimeElapsed` (+ (`self.TimeElapsed`) (`GameplayStatics.GetWorldDeltaSeconds`)))
          (`self.UpdateCameraLocation`)
          (`self.UpdateChaseMeshPosition`)
          (if (or (`self.IsPlayerOffScreenHorizontal`) (`self.IsPlayerOffScreenVertical`))
            (`PlayerController.SetViewTargetWithBlend` _returnvalue_2 _returnvalue_3 0.25 "VTBlend_Linear" 0.0 false)
            (`/Game/PGTemplate/Blueprints/Characters/Core/BP_PlatformGameCharacter.RegisterHit` _asbp_player_character (0.0 0.0 0.0) (`self.K2_GetActorLocation` _asbp_player_character) (`/Game/PGTemplate/Blueprints/Characters/Core/BP_PlatformGameCharacter.Health` _asbp_player_character))))
        (:`Finished`
          (`PlayerController.SetViewTargetWithBlend` _returnvalue (`Controller.K2_GetPawn` _returnvalue) (`self.TransitionOutTime`) "VTBlend_Linear" 0.0 false))))))

(event `self.K2_OnReset`
  (`|ExecutionSequence`
    (:`then_0`
      (goto _label :!via `Reset`))
    (:`then_1`
      (`SceneComponent.SetVisibility` (`self.ChaseObjectHandle`) false true :!label _label_3)
      (set `self.TimeElapsed` 0.0)
      (`self.UpdateCameraLocation`)
      (goto _label_2 :!via `Stop`))))

(event `self.ReceiveBeginPlay`
  (goto _label_3))

(fn `CurrentSplineLocation`
  (returns (Location :type "Vector Structure"))
  (bind _cameramotionspline (`self.CameraMotionSpline`))
  (return (`SplineComponent.GetLocationAtDistanceAlongSpline` _cameramotionspline (`KismetMathLibrary.FClamp` (* (`self.TimeElapsed`) (`self.CameraMoveSpeedSteady`)) 0.0 (`SplineComponent.GetSplineLength` _cameramotionspline)) "Local")))

(fn `IsPlayerOffScreenHorizontal`
  (returns (PlayerOffScreen :type Boolean))
  (bind _gamecamera (`self.GameCamera`))
  (bind (_returnvalue_roll _returnvalue_pitch _returnvalue_yaw) (`KismetMathLibrary.BreakRotator` (`SceneComponent.K2_GetComponentRotation` _gamecamera)))
  (bind (_returnvalue_roll_2 _returnvalue_pitch_2 _returnvalue_yaw_2) (`KismetMathLibrary.BreakRotator` (`KismetMathLibrary.FindLookAtRotation` (- (`SceneComponent.K2_GetComponentLocation` _gamecamera) (* (`SceneComponent.GetForwardVector` _gamecamera) (`CineCameraComponent.CurrentFocalLength` _gamecamera))) (`self.K2_GetActorLocation` (`Controller.K2_GetPawn` (`GameplayStatics.GetPlayerController` 0))))))
  (return (> (`KismetMathLibrary.Abs` (- _returnvalue_yaw _returnvalue_yaw_2)) (`KismetMathLibrary.Abs` (/ (`CineCameraComponent.GetHorizontalFieldOfView` _gamecamera) 2.0)))))

(fn `IsPlayerOffScreenVertical`
  (returns (PlayerOffScreen :type Boolean))
  (bind _gamecamera (`self.GameCamera`))
  (bind (_returnvalue_roll _returnvalue_pitch) (`KismetMathLibrary.BreakRotator` (`SceneComponent.K2_GetComponentRotation` _gamecamera)))
  (bind (_returnvalue_roll_2 _returnvalue_pitch_2) (`KismetMathLibrary.BreakRotator` (`KismetMathLibrary.FindLookAtRotation` (- (`SceneComponent.K2_GetComponentLocation` _gamecamera) (* (`SceneComponent.GetForwardVector` _gamecamera) (`CineCameraComponent.CurrentFocalLength` _gamecamera))) (`self.K2_GetActorLocation` (`Controller.K2_GetPawn` (`GameplayStatics.GetPlayerController` 0))))))
  (return (> (`KismetMathLibrary.Abs` (- _returnvalue_pitch _returnvalue_pitch_2)) (`KismetMathLibrary.Abs` (/ (`CineCameraComponent.GetVerticalFieldOfView` _gamecamera) 2.0)))))

(fn `LastSplineLocation`
  (returns (Location :type "Vector Structure"))
  (return (`SplineComponent.GetLocationAtDistanceAlongSpline` (`self.CameraMotionSpline`) (* (- (`self.TimeElapsed`) (`GameplayStatics.GetWorldDeltaSeconds`)) (`self.CameraMoveSpeedSteady`)) "Local")))

(fn `RelativeScreenEdgeLocations`
  (returns (Left :type "Vector Structure"))
  (bind _gamecamera (`self.GameCamera`))
  (bind (_relativelocation_x _relativelocation_y) (`KismetMathLibrary.BreakVector` (`SceneComponent.RelativeLocation` _gamecamera)))
  (return (* (+ (`KismetMathLibrary.MakeVector` 0.0 _relativelocation_y) (* (`CineCameraComponent.CurrentFocalLength` _gamecamera) (`KismetMathLibrary.NegateVector` (`SceneComponent.GetForwardVector` _gamecamera)))) (`KismetMathLibrary.DegTan` (* (`CineCameraComponent.GetHorizontalFieldOfView` _gamecamera) 0.5)))))

(fn `UpdateCameraLocation`
  (bind _location (`self.CurrentSplineLocation`))
  (bind _gamecamera (`self.GameCamera`))
  (`KismetSystemLibrary.PrintString` (`KismetStringLibrary.Conv_VectorToString` _location))
  (`SceneComponent.K2_SetRelativeLocation` _gamecamera (+ _location (`self.CameraOffsetFromSplinePoint`)) false false)
  (`SceneComponent.K2_SetRelativeRotation` _gamecamera (`self.CameraRotation`) false false))

(fn `UpdateChaseMeshPosition`
  (locals (CameraFocalOffset :type "Vector Structure" :default (0.0 0.0 0.0)) (FocalOffsetDepth :type "Float (double-precision)") (FocalOffsetHeight :type "Float (double-precision)"))
  (bind _gamecamera (`self.GameCamera`))
  (bind (_camerarotation_roll _camerarotation_pitch _camerarotation_yaw) (`KismetMathLibrary.BreakRotator` (`self.CameraRotation`)))
  (bind (_cameraoffsetfromsplinepoint_x _cameraoffsetfromsplinepoint_y) (`KismetMathLibrary.BreakVector` (`self.CameraOffsetFromSplinePoint`)))
  (bind (_cameraoffsetfromsplinepoint_x_2 _cameraoffsetfromsplinepoint_y_2) (`KismetMathLibrary.BreakVector` (`self.CameraOffsetFromSplinePoint`)))
  (bind _chaseobjecthandle (`self.ChaseObjectHandle`))
  (bind (_relativelocation_x _relativelocation_y _relativelocation_z) (`KismetMathLibrary.BreakVector` (`SceneComponent.RelativeLocation` (`self.GameCamera`))))
  (bind (_returnvalue_x _returnvalue_y _returnvalue_z) (`KismetMathLibrary.BreakVector` (`KismetMathLibrary.Normal` (- (`self.CurrentSplineLocation`) (`self.LastSplineLocation`)))))
  (bind _returnvalue (/ (`CineCameraComponent.GetHorizontalFieldOfView` (`self.GameCamera`)) 2.0))
  (bind _returnvalue_2 (/ (`CineCameraComponent.GetVerticalFieldOfView` (`self.GameCamera`)) 2.0))
  (if (!= (`self.LastSplineLocation`) (`self.CurrentSplineLocation`) :`ErrorTolerance` 0.01)
    (bind _output_get (set `local.CameraFocalOffset` (`KismetMathLibrary.NegateVector` (* (`SceneComponent.GetForwardVector` _gamecamera) (`CineCameraComponent.CurrentFocalLength` _gamecamera)))))
    (bind _returnvalue_3 (`KismetMathLibrary.VSize` _output_get))
    (set `local.FocalOffsetDepth` (* _returnvalue_3 (`KismetMathLibrary.Cos` _camerarotation_yaw)))
    (set `local.FocalOffsetHeight` (* _returnvalue_3 (`KismetMathLibrary.Cos` _camerarotation_pitch)))
    (`SceneComponent.K2_SetRelativeLocation` _chaseobjecthandle (`KismetMathLibrary.MakeVector` (- _relativelocation_x (/ (+ (`local.FocalOffsetDepth`) _cameraoffsetfromsplinepoint_y) (`KismetMathLibrary.DegTan` (`KismetMathLibrary.Lerp` (+ _camerarotation_yaw _returnvalue) (- _camerarotation_yaw _returnvalue) (+ (/ _returnvalue_x 2.0) 0.5))))) 0.0 (- _relativelocation_z (* (* (`KismetMathLibrary.DegTan` (`KismetMathLibrary.Lerp` (- _camerarotation_pitch _returnvalue_2) (+ _camerarotation_pitch _returnvalue_2) (+ (/ _returnvalue_z 2.0) 0.5))) (+ (`local.FocalOffsetDepth`) _cameraoffsetfromsplinepoint_y_2)) (`KismetMathLibrary.Lerp` 10.0 1.0 (`KismetMathLibrary.FClamp` (`self.TimeElapsed`)))))) false false)
    (`SceneComponent.K2_SetRelativeRotation` _chaseobjecthandle (`KismetMathLibrary.FindLookAtRotation` (`self.LastSplineLocation`) (`self.CurrentSplineLocation`)) false false)))

(fn `UserConstructionScript`
  (`self.UpdateCameraLocation`))