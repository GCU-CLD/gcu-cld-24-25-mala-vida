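; Fixed camera zone trigger that switches the player's view to its own cine camera while the player character is inside it.
; Entering the PlayerDetection volume blends the player controller's view target to this actor, and leaving blends it back to the character, both using BlendTime.
; The construction script pins the camera's world scale to one, so scaling the actor leaves the camera unscaled.
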(event `self.PlayerDetection.OnComponentBeginOverlap`
  (params (OverlappedComponent :type "PrimitiveComponent Object Reference") (OtherActor :type "Actor Object Reference") (OtherComp :type "PrimitiveComponent Object Reference") (OtherBodyIndex :type Integer) (bFromSweep :type Boolean) (SweepResult :type "HitResult Structure (by ref)"))
  (bind _asbp_player_character (cast `/Game/PGTemplate/Blueprints/Characters/Player/BP_PlayerCharacter` OtherActor))
  (bind _asplayer_controller (cast `PlayerController` (`Pawn.GetController` _asbp_player_character)))
  (`PlayerController.SetViewTargetWithBlend` _asplayer_controller self (`self.BlendTime`) "VTBlend_Linear" 0.0 false))

(event `self.PlayerDetection.OnComponentEndOverlap`
  (params (OverlappedComponent :type "PrimitiveComponent Object Reference") (OtherActor :type "Actor Object Reference") (OtherComp :type "PrimitiveComponent Object Reference") (OtherBodyIndex :type Integer))
  (bind _asbp_player_character (cast `/Game/PGTemplate/Blueprints/Characters/Player/BP_PlayerCharacter` OtherActor))
  (bind _asplayer_controller (cast `PlayerController` (`Pawn.GetController` _asbp_player_character)))
  (`PlayerController.SetViewTargetWithBlend` _asplayer_controller _asbp_player_character (`self.BlendTime`) "VTBlend_Linear" 0.0 false))

(fn `UserConstructionScript`
  (`SceneComponent.SetWorldScale3D` (`self.CineCamera`) (1.0 1.0 1.0)))