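; Logic-trigger object that plays a chosen Level Sequence in response to switch on/off events.
; BeginPlay creates the player from SequenceEndBehaviour (hold, ping-pong, loop, cutscene end), optionally blocking movement input.
; SwitchBehaviour decides whether switching plays and pauses, reverses direction, or only plays forward.
; Reset and initial-status changes jump playback to the matching start or end frame, disabling camera cuts during setup to avoid unwanted cuts.
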(event `self.ReceiveBeginPlay`
  (bind _moviescenesequenceloopcount (make `MovieSceneSequenceLoopCount` 0))
  (bind _sequenceendbehaviour (`self.SequenceEndBehaviour`))
  (bind _sequenceplayer (`LevelSequenceActor.SequencePlayer` (`self.SequencePlayerActor`)))
  (`|ExecutionSequence`
    (:`then_0`
      ;[1 1 1] Set up Sequence Player based on Options
      (bind _outactor (`LevelSequencePlayer.CreateLevelSequencePlayer` (`self.SequenceToPlay`) (make `MovieSceneSequencePlaybackSettings` false (select `/Game/PGTemplate/Blueprints/Objects/LogicTriggers/SequenceEndBehaviour` _sequenceendbehaviour :`NewEnumerator0` _moviescenesequenceloopcount :`NewEnumerator1` _moviescenesequenceloopcount :`NewEnumerator2` (make `MovieSceneSequenceLoopCount` -1) :`NewEnumerator3` _moviescenesequenceloopcount) 1.0 0.0 false (`self.BlockPlayerInput`) false false false false "None" (select `/Game/PGTemplate/Blueprints/Objects/LogicTriggers/SequenceEndBehaviour` _sequenceendbehaviour :`NewEnumerator0` true))))
      (set `self.SequencePlayerActor` _outactor))
    (:`then_1`
      ;[1 1 1] Bind End Behaviours
      (switch `/Game/PGTemplate/Blueprints/Objects/LogicTriggers/SequenceEndBehaviour` (`self.SequenceEndBehaviour`)
        (:`NewEnumerator1`
          (add `MovieSceneSequencePlayer.OnFinished` _sequenceplayer (delegate `PingPong`)))
        (:`NewEnumerator2`
          (add `MovieSceneSequencePlayer.OnFinished` _sequenceplayer (delegate `Loop`)))))))

(event `Loop`
  (bind _sequenceplayer (`LevelSequenceActor.SequencePlayer` (`self.SequencePlayerActor`)))
  ;[1 1 1] Bind End Behaviours
  (if (`MovieSceneSequencePlayer.IsReversed` _sequenceplayer)
    (`MovieSceneSequencePlayer.PlayReverse` _sequenceplayer)
    (else
      (`MovieSceneSequencePlayer.Play` _sequenceplayer))))

(event `PingPong`
  ;[1 1 1] Bind End Behaviours
  (`MovieSceneSequencePlayer.ChangePlaybackDirection` (`LevelSequenceActor.SequencePlayer` (`self.SequencePlayerActor`))))

(event `self.K2_OnReset`
  (bind _switchbehaviour (`self.SwitchBehaviour`))
  (bind _frametime (make `FrameTime` (make `FrameNumber` 0)))
  (bind _sequenceplayer (`LevelSequenceActor.SequencePlayer` (`self.SequencePlayerActor`)))
  (bind _sequenceplayer_2 (`LevelSequenceActor.SequencePlayer` (`self.SequencePlayerActor`)))
  (bind (_returnvalue_frame _returnvalue_framerate _returnvalue_subframe) (break `QualifiedFrameTime` (`MovieSceneSequencePlayer.GetEndTime` _sequenceplayer_2)))
  (bind _frametime_2 (make `FrameTime` _returnvalue_frame _returnvalue_subframe))
  (`parent.K2_OnReset`)
  (bind _output_get (set `self.Status` (`self.InitialStatus`) :!label _label))
  (`KismetSystemLibrary.DelayUntilNextTick`)
  ;[1 1 1] Disable Camera Cuts to prevent trigger during setup
  (`MovieSceneSequencePlayer.SetDisableCameraCuts` (`LevelSequenceActor.SequencePlayer` (`self.SequencePlayerActor`)) true)
  ;[1 1 1] Set Starting Status Appropriately
  (if (`self.Status`)
    (switch `/Game/PGTemplate/Blueprints/Objects/LogicTriggers/SequenceBehaviour` _switchbehaviour ; Init ON
      (:`NewEnumerator0`
        _)
      (:`NewEnumerator1`
        _))
    (`MovieSceneSequencePlayer.Play` _sequenceplayer)
    (else
      (switch `/Game/PGTemplate/Blueprints/Objects/LogicTriggers/SequenceBehaviour` _switchbehaviour ; Init OFF
        (:`NewEnumerator0`
          _)
        (:`NewEnumerator1`
          _))
      (`MovieSceneSequencePlayer.PlayReverse` _sequenceplayer)
      (switch `/Game/PGTemplate/Blueprints/Objects/LogicTriggers/SequenceEndBehaviour` (`self.SequenceEndBehaviour`)
        (:`NewEnumerator0`
          (`MovieSceneSequencePlayer.Stop` _sequenceplayer)))))
  ;[1 1 1] Jump to appriopriate starting frame
  (`MovieSceneSequencePlayer.SetPlaybackPosition` _sequenceplayer_2 (make `MovieSceneSequencePlaybackParams` (select `bool` _output_get :`false` _frametime :`true` (select `/Game/PGTemplate/Blueprints/Objects/LogicTriggers/SequenceBehaviour` (`self.SwitchBehaviour`) :`NewEnumerator0` _frametime_2 :`NewEnumerator1` _frametime_2 :`NewEnumerator2` _frametime)) 0.0 "" (struct) "Frame" "Jump" true))
  ;[1 1 1] Re-enable Camera Cuts
  (`MovieSceneSequencePlayer.SetDisableCameraCuts` (`LevelSequenceActor.SequencePlayer` (`self.SequencePlayerActor`)) false))

(event `/Game/PGTemplate/Blueprints/Objects/Switches/Core/SwitchInterface.SetInitialStatus`
  (params (InitialStatus :type Boolean))
  (set `self.InitialStatus` InitialStatus)
  (goto _label))

(event `/Game/PGTemplate/Blueprints/Objects/Switches/Core/SwitchInterface.SwitchOn`
  (bind _sequenceplayer (`LevelSequenceActor.SequencePlayer` (`self.SequencePlayerActor`)))
  (switch `/Game/PGTemplate/Blueprints/Objects/LogicTriggers/SequenceBehaviour` (`self.SwitchBehaviour`)
    (:`NewEnumerator0`
      (`MovieSceneSequencePlayer.Play` _sequenceplayer :!label _label_2))
    (:`NewEnumerator1`
      (`MovieSceneSequencePlayer.ChangePlaybackDirection` _sequenceplayer :!label _label_3))
    (:`NewEnumerator2`
      (goto _label_2))))

(event `/Game/PGTemplate/Blueprints/Objects/Switches/Core/SwitchInterface.SwitchOff`
  (switch `/Game/PGTemplate/Blueprints/Objects/LogicTriggers/SequenceBehaviour` (`self.SwitchBehaviour`)
    (:`NewEnumerator0`
      (`MovieSceneSequencePlayer.Pause` (`LevelSequenceActor.SequencePlayer` (`self.SequencePlayerActor`))))
    (:`NewEnumerator1`
      (goto _label_3))))

(fn `DoSequencePlayerBehaviour`
  (params (Selection :type "/Game/PGTemplate/Blueprints/Objects/LogicTriggers/SequenceBehaviour Enum" :default "NewEnumerator0"))
  (bind _sequenceplayer (`LevelSequenceActor.SequencePlayer` (`self.SequencePlayerActor`)))
  (bind _sequenceplayer_2 (`LevelSequenceActor.SequencePlayer` (`self.SequencePlayerActor`)))
  (bind _sequenceplayer_3 (`LevelSequenceActor.SequencePlayer` (`self.SequencePlayerActor`)))
  (bind _returnvalue (`MovieSceneSequencePlayer.IsPlaying` _sequenceplayer))
  (switch `/Game/PGTemplate/Blueprints/Objects/LogicTriggers/SequenceBehaviour` Selection
    (:`NewEnumerator0`
      (if _returnvalue
        (if (`MovieSceneSequencePlayer.IsReversed` _sequenceplayer)
          (`MovieSceneSequencePlayer.Play` (`LevelSequenceActor.SequencePlayer` (`self.SequencePlayerActor`)) :!label _label))
        (else
          (goto _label))))
    (:`NewEnumerator1`
      (if _returnvalue
        (`MovieSceneSequencePlayer.Pause` (`LevelSequenceActor.SequencePlayer` (`self.SequencePlayerActor`)))))
    (:`NewEnumerator2`
      (if (`MovieSceneSequencePlayer.IsPlaying` _sequenceplayer_2)
        (if (`MovieSceneSequencePlayer.IsReversed` _sequenceplayer_2)
          (`MovieSceneSequencePlayer.Play` _sequenceplayer_3)
          (else
            (`MovieSceneSequencePlayer.PlayReverse` _sequenceplayer_3 :!label _label_2)))
        (else
          (goto _label_2))))))

(fn `GetStatus`
  (returns (isOn :type Boolean))
  (return (`self.Status`)))

(fn `UserConstructionScript`)