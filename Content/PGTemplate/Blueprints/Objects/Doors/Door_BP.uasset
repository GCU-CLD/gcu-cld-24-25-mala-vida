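; Door actor that swings open and closed in response to switch events and reports whether it is open.
; Switchon and SwitchOff check the IsOpen flag, play an open or close sound, and play or reverse a timeline that drives the door mesh's relative yaw.
; SetInitialStatus jumps the timeline to its start or end and applies the rotation without sound, while GetStatus returns IsOpen.
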(event `/Game/PGTemplate/Blueprints/Objects/Switches/Core/SwitchInterface.SwitchOn`
  (if (not (`self.isOpen`))
    (`GameplayStatics.PlaySoundAtLocation` "/Game/PGTemplate/Blueprints/Characters/Core/Audio/Door-Open_Cue.Door-Open_Cue" (`self.K2_GetActorLocation`) (struct) 1.0 1.0 0.0 null null null null)
    (set `self.isOpen` true)
    (bind (_direction _doorrotation) (`Timeline|Timeline` :!label _label)
      (:`Update`
        (`SceneComponent.K2_SetRelativeRotation` (`self.Door`) (`KismetMathLibrary.MakeRotator` 0.0 0.0 _doorrotation) false false :!label _label_2)))))

(event `/Game/PGTemplate/Blueprints/Objects/Switches/Core/SwitchInterface.SwitchOff`
  (if (`self.isOpen`)
    (`GameplayStatics.PlaySoundAtLocation` "/Game/PGTemplate/Blueprints/Characters/Core/Audio/Door-Close_Cue.Door-Close_Cue" (`self.K2_GetActorLocation`) (struct) 1.0 1.0 0.0 null null null null)
    (set `self.isOpen` false)
    (goto _label :!via `Reverse`)))

(event `/Game/PGTemplate/Blueprints/Objects/Switches/Core/SwitchInterface.SetInitialStatus`
  (params (InitialStatus :type Boolean))
  (bind _timeline (`self.Timeline`))
  (bind _output_get (set `self.isOpen` InitialStatus))
  (`TimelineComponent.SetNewTime` _timeline (`KismetMathLibrary.SelectFloat` (`TimelineComponent.GetTimelineLength` _timeline) 0.0 _output_get))
  (goto _label_2))

(fn `GetStatus`
  (returns (isOn :type Boolean))
  (return (`self.isOpen`)))

(fn `UserConstructionScript`)