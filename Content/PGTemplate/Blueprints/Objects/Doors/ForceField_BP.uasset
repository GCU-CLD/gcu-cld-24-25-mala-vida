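; Switchable force field barrier that toggles its visibility, collision and sound through Switchon and SwitchOff events.
; The construction script builds a quad between the actor origin and EndPoint with Geometry Script, using complex-as-simple collision and a colour-tinted dynamic material.
; InvertBehaviour flips the switch events, initial status and reported status, so a switch-on signal can lower the field instead of raising it.
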(event `/Game/PGTemplate/Blueprints/Objects/Core/SwitchInterface.SwitchOn`
  (bind _returnvalue (`self.K2_GetActorLocation`))
  (bind _ison (`self.isOn`))
  (bind _forcefieldmeshcomponent (`self.ForceFieldMeshComponent`))
  (bind _ff_on_cue (`self.FF_On_Cue`))
  (if (`self.InvertBehaviour`)
    (if _ison :!label _label
      (`GameplayStatics.PlaySoundAtLocation` "/Game/PGTemplate/Blueprints/Characters/Core/Audio/FF_On_Cue.FF_On_Cue" _returnvalue (struct) 1.0 1.0 0.0 null null null null)
      (`SceneComponent.SetVisibility` _forcefieldmeshcomponent false false)
      (`PrimitiveComponent.SetCollisionEnabled` _forcefieldmeshcomponent "NoCollision")
      (set `self.isOn` false)
      (`AudioComponent.Stop` _ff_on_cue))
    (else
      (if (not _ison) :!label _label_2
        (`GameplayStatics.PlaySoundAtLocation` "/Game/PGTemplate/Blueprints/Characters/Core/Audio/FF_On_Cue.FF_On_Cue" _returnvalue (struct) 1.0 1.0 0.0 null null null null)
        (`SceneComponent.SetVisibility` _forcefieldmeshcomponent true false)
        (`PrimitiveComponent.SetCollisionEnabled` _forcefieldmeshcomponent "QueryAndPhysics")
        (set `self.isOn` true)
        (`AudioComponent.Play` _ff_on_cue 0.0)))))

(event `/Game/PGTemplate/Blueprints/Objects/Core/SwitchInterface.SwitchOff`
  (if (`self.InvertBehaviour`)
    (goto _label_2)
    (else
      (goto _label))))

(event `/Game/PGTemplate/Blueprints/Objects/Core/SwitchInterface.SetInitialStatus`
  (params (InitialStatus :type Boolean))
  (bind _forcefieldmeshcomponent (`self.ForceFieldMeshComponent`))
  (bind _returnvalue (select `bool` (`self.InvertBehaviour`) :`false` InitialStatus :`true` (not InitialStatus)))
  (`SceneComponent.SetVisibility` _forcefieldmeshcomponent _returnvalue false)
  (`PrimitiveComponent.SetCollisionEnabled` _forcefieldmeshcomponent (select `bool` _returnvalue :`false` "NoCollision" :`true` "QueryAndPhysics" :!type "ECollisionEnabled Enum"))
  (set `self.isOn` _returnvalue))

(fn `GetStatus`
  (returns (isOn :type Boolean))
  (bind _ison (`self.isOn`))
  (return (select `bool` (`self.InvertBehaviour`) :`false` _ison :`true` (not _ison))))

(fn `UserConstructionScript`
  (bind _endpoint (`self.EndPoint`))
  (bind _forcefieldmeshcomponent (`self.ForceFieldMeshComponent`))
  (bind _returnvalue (`KismetMathLibrary.Abs` (`KismetMathLibrary.VSize` _endpoint)))
  (bind _returnvalue_2 (`KismetMathLibrary.SelectFloat` 100.0 -100.0 (> (.x _endpoint) 0.0)))
  (`SceneComponent.K2_SetRelativeLocation` (`self.End`) _endpoint false false)
  (bind _returnvalue_3 (`BaseDynamicMeshComponent.GetDynamicMesh` (`self.ForceFieldMeshComponent`)))
  (`GeometryScriptLibrary_MeshPrimitiveFunctions.AppendTriangulatedPolygon` _returnvalue_3 (struct) (`KismetMathLibrary.MakeTransform` (0.0 0.0 0.0) (`KismetMathLibrary.FindLookAtRotation` (0.0 0.0 0.0) (`self.EndPoint`))) (`|MakeArray` (0.0 0.0) (`KismetMathLibrary.MakeVector2D` 0.0 _returnvalue_2) (`KismetMathLibrary.MakeVector2D` _returnvalue _returnvalue_2) (`KismetMathLibrary.MakeVector2D` _returnvalue) :!type "Vector2D Structure") true null)
  (bind _returnvalue_4 (`KismetMaterialLibrary.CreateDynamicMaterialInstance` "/Game/PGTemplate/Blueprints/Objects/Doors/Materials/ForceFieldMaterial.ForceFieldMaterial"))
  (`PrimitiveComponent.SetMaterial` (`self.ForceFieldMeshComponent`) 0 _returnvalue_4)
  (`MaterialInstanceDynamic.SetVectorParameterValue` _returnvalue_4 "Colour" (`self.Colour`))
  (`DynamicMeshComponent.SetComplexAsSimpleCollisionEnabled` _forcefieldmeshcomponent true true)
  (`PrimitiveComponent.SetCollisionEnabled` _forcefieldmeshcomponent "QueryAndPhysics"))