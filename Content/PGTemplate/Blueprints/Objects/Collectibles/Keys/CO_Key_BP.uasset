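; CO_Key_BP is a collectible key Blueprint whose appearance follows its Colour setting of red, green or blue.
; Its construction script calls the parent's, then creates a dynamic instance of Key_M, sets the Colour vector parameter from that selection and applies it to CollectibleMesh.
; The event graph holds only disabled placeholder events, so this Blueprint adds no runtime logic of its own.
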(fn `UserConstructionScript`
  (`parent.UserConstructionScript`)
  (bind _returnvalue (`KismetMaterialLibrary.CreateDynamicMaterialInstance` "/Game/PGTemplate/Blueprints/Objects/Collectibles/Keys/Materials/Key_M.Key_M"))
  (`MaterialInstanceDynamic.SetVectorParameterValue` _returnvalue "Colour" (select `/Game/PGTemplate/Blueprints/Objects/Collectibles/Keys/KeyColours` (`self.Colour`) :`NewEnumerator0` (struct :`R` 1.0 :`A` 1.0) :`NewEnumerator1` (struct :`G` 1.0 :`A` 1.0) :`NewEnumerator2` (struct :`B` 1.0 :`A` 1.0) :!type "LinearColor Structure"))
  (`PrimitiveComponent.SetMaterial` (`self.CollectibleMesh`) 0 _returnvalue))