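; IO_Lock_BP is an interactable lock switch that only activates when the character holds its required object.
; Interact retrieves that object from inventory and runs the parent interaction, then the character puts it away in PostSwitchActions.
; Without it, control is briefly blocked while a head-shake montage plays.
; Highlighting creates a requirement widget showing the object's name on RequirementIndicator, and de-highlighting clears it.
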(event `self.ReceiveBeginPlay`
  (`parent.ReceiveBeginPlay`)
  (bind _aslock_requirements_w (cast `/Game/PGTemplate/Blueprints/Objects/Switches/Materials/LockRequirements_W` (`WidgetComponent.GetWidget` (`self.RequirementIndicator`)))))

(event `/Game/PGTemplate/Blueprints/Objects/Core/InteractionObject_BP.Highlight`
  (params (Character :type "/Game/PGTemplate/Blueprints/Characters/Core/BP_PlatformGameCharacter Object Reference") (HighlightColor :type "LinearColor Structure"))
  (bind _returnvalue (`|CreateWidget` "/Game/PGTemplate/Blueprints/Objects/Switches/Materials/LockRequirements_W.LockRequirements_W_C" null null (`/Game/PGTemplate/Blueprints/Objects/Collectibles/Core/IO_CollectibleObject_BP.ObjectName` (`self.RequiredObject`))))
  (`WidgetComponent.SetWidget` (`self.RequirementIndicator`) _returnvalue)
  (`parent.Highlight` Character HighlightColor))

(event `self.PostSwitchActions`
  (params (InstigatingCharacter :type "/Game/PGTemplate/Blueprints/Characters/Core/BP_PlatformGameCharacter Object Reference"))
  (`/Game/PGTemplate/Blueprints/Characters/Player/BP_PlayerCharacter.PutAway` InstigatingCharacter))

(event `/Game/PGTemplate/Blueprints/Objects/Core/InteractionObject_BP.DeHighlight`
  (params (Character :type "/Game/PGTemplate/Blueprints/Characters/Core/BP_PlatformGameCharacter Object Reference"))
  (`WidgetComponent.SetWidget` (`self.RequirementIndicator`) null)
  (`parent.DeHighlight` Character))

(event `/Game/PGTemplate/Blueprints/Objects/Core/InteractionObject_BP.Interact`
  (params (InstigatingCharacter :type "/Game/PGTemplate/Blueprints/Characters/Core/BP_PlatformGameCharacter Object Reference"))
  (bind _requiredobject (`self.RequiredObject`))
  (bind _objectfound (`/Game/PGTemplate/Blueprints/Characters/Player/BP_PlayerCharacter.CheckInventory` InstigatingCharacter _requiredobject))
  (if _objectfound
    (`/Game/PGTemplate/Blueprints/Characters/Player/BP_PlayerCharacter.RetrieveFromInventory` InstigatingCharacter _requiredobject)
    (`parent.Interact` InstigatingCharacter)
    (else
      (set `/Game/PGTemplate/Blueprints/Characters/Player/BP_PlayerCharacter.LookAtAlpha` 0.0 InstigatingCharacter)
      (`/Game/PGTemplate/Blueprints/Characters/Player/BP_PlayerCharacter.BlockControl` InstigatingCharacter false)
      (bind _returnvalue (`Character.PlayAnimMontage` InstigatingCharacter "/Game/PGTemplate/Blueprints/Characters/Core/Animations/Mixamo/Interactions/ThoughtfulHeadShake_UE_Montage.ThoughtfulHeadShake_UE_Montage" 2.0 "None"))
      (`KismetSystemLibrary.Delay` (/ _returnvalue 2.0))
      (`/Game/PGTemplate/Blueprints/Characters/Player/BP_PlayerCharacter.UnBlockControl` InstigatingCharacter))))

(fn `UserConstructionScript`
  (bind _requiredobject (`self.RequiredObject`))
  (bind (_aslock_requirements_w _bsuccess) (cast `/Game/PGTemplate/Blueprints/Objects/Switches/Materials/LockRequirements_W` (`WidgetComponent.GetWidget` (`self.RequirementIndicator`)) :!pure true))
  (`parent.UserConstructionScript`)
  (`/Engine/EditorBlueprintResources/StandardMacros.IsValid` _requiredobject
    (:`Is Valid`
      (if _bsuccess
        (set `/Game/PGTemplate/Blueprints/Objects/Switches/Materials/LockRequirements_W.ObjectName` (`/Game/PGTemplate/Blueprints/Objects/Collectibles/Core/IO_CollectibleObject_BP.ObjectName` _requiredobject) _aslock_requirements_w)))))