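; Switch cable Blueprint that draws a spline-shaped cable coloured green when on and red when off.
; The construction script tiles spline mesh segments along CableSpline at SegmentSize intervals, all sharing one dynamic material instance.
; SetInitialStatus, Switchon and SwitchOff set IsOn and update that material's Colour parameter, while GetStatus returns the state.
; OnReset only reapplies the colour for the current state.
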(event `self.K2_OnReset`
  (`MaterialInstanceDynamic.SetVectorParameterValue` (`self.CableMaterial`) "Colour" (`KismetMathLibrary.SelectColor` (struct :`G` 1.0 :`A` 1.0) (struct :`R` 1.0 :`A` 1.0) (`self.isOn`)) :!label _label))

(event `/Game/PGTemplate/Blueprints/Objects/Switches/Core/SwitchInterface.SetInitialStatus`
  (params (InitialStatus :type Boolean))
  (set `self.isOn` InitialStatus)
  (goto _label))

(event `/Game/PGTemplate/Blueprints/Objects/Switches/Core/SwitchInterface.SwitchOn`
  (if (not (`self.isOn`))
    (set `self.isOn` true)
    (goto _label)))

(event `/Game/PGTemplate/Blueprints/Objects/Switches/Core/SwitchInterface.SwitchOff`
  (if (`self.isOn`)
    (set `self.isOn` false)
    (goto _label)))

(fn `GetStatus`
  (returns (isOn :type Boolean))
  (return (`self.isOn`)))

(fn `UserConstructionScript`
  (bind _cablespline (`self.CableSpline`))
  (bind _segmentsize (`self.SegmentSize`))
  (`|ExecutionSequence`
    (:`then_0`
      (bind _returnvalue (`KismetMaterialLibrary.CreateDynamicMaterialInstance` "/Game/PGTemplate/Blueprints/Objects/Switches/Materials/Cable_M.Cable_M"))
      (set `self.CableMaterial` _returnvalue)
      (for _index (range (+ (`KismetMathLibrary.FFloor` (/ (`SplineComponent.GetSplineLength` (`self.CableSpline`)) (`self.SegmentSize`))) 1))
        (bind _returnvalue_2 (`AddComponent|NODE_AddSplineMeshComponent-0`))
        (`StaticMeshComponent.SetStaticMesh` _returnvalue_2 "/Game/PGTemplate/Blueprints/Objects/Switches/Meshes/cable.cable")
        (bind _returnvalue_3 (* _index _segmentsize))
        (bind _returnvalue_4 (* _segmentsize (+ _index 1)))
        (bind _returnvalue_5 (`KismetMathLibrary.FClamp` _returnvalue_4 _returnvalue_4 (`SplineComponent.GetSplineLength` (`self.CableSpline`))))
        (`SplineMeshComponent.SetStartAndEnd` _returnvalue_2 (`SplineComponent.GetLocationAtDistanceAlongSpline` _cablespline _returnvalue_3 "Local") (`SplineComponent.GetTangentAtDistanceAlongSpline` _cablespline _returnvalue_3 "Local") (`SplineComponent.GetLocationAtDistanceAlongSpline` _cablespline _returnvalue_5 "Local") (`SplineComponent.GetTangentAtDistanceAlongSpline` _cablespline _returnvalue_5 "Local") true)
        (`PrimitiveComponent.SetMaterial` _returnvalue_2 0 (`self.CableMaterial`))))
    (:`then_1`
      (`MaterialInstanceDynamic.SetVectorParameterValue` (`self.CableMaterial`) "Colour" (`KismetMathLibrary.SelectColor` (struct :`G` 1.0 :`A` 1.0) (struct :`R` 1.0 :`A` 1.0) (`self.isOn`))))))