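; Invisible trigger switch that toggles its state and updates targeted actors when a character enters or leaves its PlayerDetection volume.
; It responds to the player, and also to other platform game characters when TriggeredByEnemies is set.
; TriggerBehaviour selects on-while-present, off-while-present, or trigger-once, which only turns on at overlap begin, ignores exit, and has no guard against refiring.
; State changes call UpdateTargetedActors to propagate SwitchIsOn.
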(event `self.PlayerDetection.OnComponentBeginOverlap`
  (params (OverlappedComponent :type "PrimitiveComponent Object Reference") (OtherActor :type "Actor Object Reference") (OtherComp :type "PrimitiveComponent Object Reference") (OtherBodyIndex :type Integer) (bFromSweep :type Boolean) (SweepResult :type "HitResult Structure (by ref)"))
  (bind _switchison (`self.SwitchIsOn`))
  (cast `/Game/PGTemplate/Blueprints/Characters/Player/BP_PlayerCharacter` OtherActor
    (:`then`
      (switch `/Game/PGTemplate/Blueprints/Objects/Switches/Materials/InvisibleTriggerBehaviour` (`self.TriggerBehaviour`) :!label _label
        (:`NewEnumerator0`
          (if (not _switchison)
            (set `self.SwitchIsOn` true)
            (`self.UpdateTargetedActors` :!label _label_2)))
        (:`NewEnumerator1`
          (if _switchison
            (set `self.SwitchIsOn` false)
            (goto _label_2)))
        (:`NewEnumerator2`
          (set `self.SwitchIsOn` true)
          (goto _label_2))))
    (:`CastFailed`
      (if (`self.TriggeredByEnemies`)
        (cast `/Game/PGTemplate/Blueprints/Characters/Core/BP_PlatformGameCharacter` OtherActor)
        (goto _label)))))

(event `self.PlayerDetection.OnComponentEndOverlap`
  (params (OverlappedComponent :type "PrimitiveComponent Object Reference") (OtherActor :type "Actor Object Reference") (OtherComp :type "PrimitiveComponent Object Reference") (OtherBodyIndex :type Integer))
  (bind _switchison (`self.SwitchIsOn`))
  (cast `/Game/PGTemplate/Blueprints/Characters/Player/BP_PlayerCharacter` OtherActor
    (:`then`
      (switch `/Game/PGTemplate/Blueprints/Objects/Switches/Materials/InvisibleTriggerBehaviour` (`self.TriggerBehaviour`) :!label _label_3
        (:`NewEnumerator0`
          (if _switchison
            (set `self.SwitchIsOn` false)
            (`self.UpdateTargetedActors` :!label _label_4)))
        (:`NewEnumerator1`
          (if (not _switchison)
            (set `self.SwitchIsOn` true)
            (goto _label_4)))))
    (:`CastFailed`
      (if (`self.TriggeredByEnemies`)
        (cast `/Game/PGTemplate/Blueprints/Characters/Core/BP_PlatformGameCharacter` OtherActor)
        (goto _label_3)))))

(fn `UserConstructionScript`
  (`parent.UserConstructionScript`))