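; Mantle spot actor that registers itself with platform game characters entering its detection volume and forces enemies to mantle.
; Construction places entry, exit, climb and hand-anchor points from position vectors, adds guide arrows and floor-snaps entry and exit by line trace.
; BeginPlay resets the climb point to the raw exit vector; end overlap unregisters only players.
; Helpers check for a blocked exit and temporarily freeze overlapping non-character physics objects.
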(event `self.ReceiveBeginPlay`
  (bind (_exitposition_x _exitposition_y _exitposition_z) (`KismetMathLibrary.BreakVector` (`self.ExitPosition`)))
  (bind _output_get (set `self.ClimbPosition` (`KismetMathLibrary.MakeVector` _exitposition_x _exitposition_y _exitposition_z)))
  (`SceneComponent.K2_SetRelativeLocation` (`self.PlayerClimbPosition`) _output_get false false))

(event `self.PlayerDetection.OnComponentBeginOverlap`
  (params (OverlappedComponent :type "PrimitiveComponent Object Reference") (OtherActor :type "Actor Object Reference") (OtherComp :type "PrimitiveComponent Object Reference") (OtherBodyIndex :type Integer) (bFromSweep :type Boolean) (SweepResult :type "HitResult Structure (by ref)"))
  (bind _asbp_platform_game_character (cast `/Game/PGTemplate/Blueprints/Characters/Core/BP_PlatformGameCharacter` OtherActor))
  (`/Game/PGTemplate/Blueprints/Characters/Player/BP_PlayerCharacter.AddNewMantleSpot` _asbp_platform_game_character self)
  (bind _asbp_enemy_base (cast `/Game/PGTemplate/Blueprints/Characters/Enemy/Core/BP_Enemy_Base` _asbp_platform_game_character))
  (`/Game/PGTemplate/Blueprints/Characters/Enemy/Core/BP_Enemy_Base.ForceMantle` _asbp_enemy_base))

(event `self.PlayerDetection.OnComponentEndOverlap`
  (params (OverlappedComponent :type "PrimitiveComponent Object Reference") (OtherActor :type "Actor Object Reference") (OtherComp :type "PrimitiveComponent Object Reference") (OtherBodyIndex :type Integer))
  (bind _asbp_player_character (cast `/Game/PGTemplate/Blueprints/Characters/Player/BP_PlayerCharacter` OtherActor))
  (`/Game/PGTemplate/Blueprints/Characters/Player/BP_PlayerCharacter.RemoveMantleSpot` _asbp_player_character self))

(event `LockPhysicsObjects`
  (for _array_element (`PrimitiveComponent.GetOverlappingComponents` (`self.PlayerDetection`))
    (cast `/Game/PGTemplate/Blueprints/Characters/Core/BP_PlatformGameCharacter` (`ActorComponent.GetOwner` _array_element)
      (:`CastFailed`
        (if (`SceneComponent.IsSimulatingPhysics` _array_element "None")
          (`KismetArrayLibrary.Array_Add` (`self.LockedPhysicsComponents`) _array_element)
          (`PrimitiveComponent.SetSimulatePhysics` _array_element false))))))

(event `UnlockPhysicsObjects`
  (for _array_element (`self.LockedPhysicsComponents`)
    (`PrimitiveComponent.SetSimulatePhysics` _array_element true)))

(fn `AddArrowToComponent`
  (params (Parent :type "SceneComponent Object Reference") (Scale :type "Vector Structure" :default (1.0 1.0 1.0)) (Colour :type "LinearColor Structure" :default (struct :`R` 1.0 :`A` 1.0)))
  (bind _returnvalue (`AddComponent|NODE_AddArrowComponent-0`))
  (`SceneComponent.SetWorldScale3D` _returnvalue Scale)
  (`ArrowComponent.SetArrowColor` _returnvalue Colour)
  (`SceneComponent.K2_AttachToComponent` _returnvalue Parent "None" "SnapToTarget" "SnapToTarget" "KeepWorld" true))

(fn `DropSceneComponentToFloor`
  (params (SceneComponent :type "SceneComponent Object Reference"))
  (bind _returnvalue (`SceneComponent.K2_GetComponentLocation` SceneComponent))
  (bind _outhit (`KismetSystemLibrary.LineTraceSingle` (+ _returnvalue (`KismetMathLibrary.MakeVector` 0.0 0.0 (.z (`.BoxExtent` (`KismetSystemLibrary.GetComponentBounds` (`self.PlayerDetection`)))))) (+ _returnvalue (0.0 0.0 -1000000.0)) "TraceTypeQuery1"))
  (`SceneComponent.K2_SetWorldLocation` SceneComponent (`.Location` (`GameplayStatics.BreakHitResult` _outhit)) false false))

(fn `ExitBlocked`
  (returns (ExitBlocked :type Boolean))
  (bind (_outcomponents _returnvalue) (`KismetSystemLibrary.BoxOverlapComponents` (+ (`SceneComponent.K2_GetComponentLocation` (`self.PlayerExit`)) (0.0 0.0 20.0)) (10.0 10.0 10.0) (`|MakeArray` "ObjectTypeQuery1" "ObjectTypeQuery2" "ObjectTypeQuery3" "ObjectTypeQuery4" :!type "EObjectTypeQuery Enum") null (`|MakeArray` self :!type "Actor Object Reference")))
  (return _returnvalue))

(fn `UserConstructionScript`
  (`|ExecutionSequence`
    (:`then_0`
      ;[1 1 1] Add Guide Arows to Scene Positions for Entry/Exit
      (`self.AddArrowToComponent` (`self.PlayerEntry`))
      (`self.AddArrowToComponent` (`self.PlayerExit`))
      (`self.AddArrowToComponent` (`self.PlayerClimbPosition`)))
    (:`then_1`
      ;[1 1 1] Use Entry/Exit Position Vectors w/ Handles to position Scene Components
      (`SceneComponent.K2_SetRelativeLocation` (`self.PlayerEntry`) (`self.EntryPosition`) false false)
      (`SceneComponent.K2_SetRelativeLocation` (`self.PlayerExit`) (`self.ExitPosition`) false false)
      (`SceneComponent.K2_SetRelativeLocation` (`self.PlayerClimbPosition`) (`self.ClimbPosition`) false false)
      (`SceneComponent.K2_SetRelativeLocation` (`self.HandAnchor`) (`self.HandAnchorPosition`) false false))
    (:`then_2`
      ;[1 1 1] Drop Scene Components to Floor
      (`self.DropSceneComponentToFloor` (`self.PlayerEntry`))
      (`self.DropSceneComponentToFloor` (`self.PlayerExit`)))))