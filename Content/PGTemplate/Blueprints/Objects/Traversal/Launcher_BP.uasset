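; Traversal launcher that throws the platformer character toward an editable destination point when it overlaps while active.
; It computes a suggested projectile velocity, boosts it for LaunchCharacter, then plays smoke and a timeline that moves the indicator vertically.
; IO_Switch_BP actors can target it through on, off and initial-status events, with a dynamic material showing green or red.
; At BeginPlay it turns itself on if no switch targets it.
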(event `self.CharacterDetection.OnComponentBeginOverlap`
  (params (OverlappedComponent :type "PrimitiveComponent Object Reference") (OtherActor :type "Actor Object Reference") (OtherComp :type "PrimitiveComponent Object Reference") (OtherBodyIndex :type Integer) (bFromSweep :type Boolean) (SweepResult :type "HitResult Structure (by ref)"))
  (if (`self.isActive`)
    (bind _asbp_platform_game_character (cast `/Game/PGTemplate/Blueprints/Characters/Core/BP_PlatformGameCharacter` OtherActor))
    (bind _tossvelocity (`GameplayStatics.BlueprintSuggestProjectileVelocity` (`self.K2_GetActorLocation` _asbp_platform_game_character) (+ (`self.K2_GetActorLocation`) (`KismetMathLibrary.GreaterGreater_VectorRotator` (`self.DestinationPoint`) (`self.K2_GetActorRotation`))) 1000.0 0.0 "DoNotTrace"))
    (`Character.LaunchCharacter` _asbp_platform_game_character (* _tossvelocity 1.5) true true)
    (`ActorComponent.Activate` (`self.LauncherSmoke_NS`) true)
    (bind (_direction _z_motion) (`Timeline|Timeline` :!via `PlayFromStart`)
      (:`Update`
        (`SceneComponent.K2_SetRelativeLocation` (`self.Indicator`) (+ (0.0 0.0 50.0) (`KismetMathLibrary.MakeVector` 0.0 0.0 _z_motion)) false false)))))

(event `/Game/PGTemplate/Blueprints/Objects/Core/SwitchInterface.SwitchOn`
  (set `self.isActive` true)
  (`MaterialInstanceDynamic.SetVectorParameterValue` (`self.IndicatorMaterial`) "Colour" (struct :`G` 1.0 :`A` 1.0)))

(event `/Game/PGTemplate/Blueprints/Objects/Core/SwitchInterface.SwitchOff`
  (set `self.isActive` false)
  (`MaterialInstanceDynamic.SetVectorParameterValue` (`self.IndicatorMaterial`) "Colour" (struct :`R` 1.0 :`A` 1.0)))

(event `/Game/PGTemplate/Blueprints/Objects/Core/SwitchInterface.SetInitialStatus`
  (params (InitialStatus :type Boolean))
  (set `self.isActive` InitialStatus)
  (`MaterialInstanceDynamic.SetVectorParameterValue` (`self.IndicatorMaterial`) "Colour" (`KismetMathLibrary.SelectColor` (struct :`G` 1.0 :`A` 1.0) (struct :`R` 1.0 :`A` 1.0) (`self.isActive`))))

(event `self.ReceiveBeginPlay`
  (`parent.ReceiveBeginPlay`)
  (if (not (`self.IsTargetedBySwitch`))
    (`self.SwitchOn`)))

(fn `GetStatus`
  (returns (isOn :type Boolean))
  (return (`self.isActive`)))

(fn `IsTargetedBySwitch`
  (returns (IsTargetedBySwitch :type Boolean))
  (locals (IsTargetedBySwitchLocal :type Boolean))
  (set `local.IsTargetedBySwitchLocal` false)
  (bind _outactors (`GameplayStatics.GetAllActorsOfClass` "/Game/PGTemplate/Blueprints/Objects/Switches/IO_Switch_BP.IO_Switch_BP_C"))
  (for _array_element _outactors
    (for _array_element_2 (`/Game/PGTemplate/Blueprints/Objects/Switches/IO_Switch_BP.TargetedActors` _array_element)
      (if (== _array_element_2 self)
        (set `local.IsTargetedBySwitchLocal` true))))
  (return (`local.IsTargetedBySwitchLocal`)))

(fn `UserConstructionScript`
  (`SceneComponent.K2_SetRelativeLocation` (`self.DestinationMarker`) (`self.DestinationPoint`) false false)
  (bind _returnvalue (`KismetMaterialLibrary.CreateDynamicMaterialInstance` "/Game/PGTemplate/Environments/Materials/BasicColouredMaterial_M.BasicColouredMaterial_M"))
  (bind _output_get (set `self.IndicatorMaterial` _returnvalue))
  (`PrimitiveComponent.SetMaterial` (`self.Indicator`) 0 _output_get)
  (`MaterialInstanceDynamic.SetVectorParameterValue` _output_get "Colour" (`KismetMathLibrary.SelectColor` (struct :`G` 1.0 :`A` 1.0) (struct :`R` 1.0 :`A` 1.0) (`self.isActive`))))