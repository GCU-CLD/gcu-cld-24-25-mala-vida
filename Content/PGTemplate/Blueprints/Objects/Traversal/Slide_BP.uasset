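; Traversal slide actor that carries an overlapping platformer character along a straight path to the SlideEnd point.
; The construction script stretches and angles the detection volume toward SlideEnd, using a downward trace to set its height.
; On overlap, it blocks input, switches the character to Flying and plays a montage while a timeline lerps its position, rate-scaled by remaining distance and SlideSpeed.
; Finishing or StopSliding restores input and sets Falling.
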(event `self.ReceiveBeginPlay`
  (`TimelineComponent.SetPlayRate` (`self.SlidePositionLerp`) (/ 1.0 (/ (`KismetMathLibrary.VSize` (`self.SlideEnd`)) (`self.SlideSpeed`)))))

(event `self.PlayerDetection.OnComponentBeginOverlap`
  (params (OverlappedComponent :type "PrimitiveComponent Object Reference") (OtherActor :type "Actor Object Reference") (OtherComp :type "PrimitiveComponent Object Reference") (OtherBodyIndex :type Integer) (bFromSweep :type Boolean) (SweepResult :type "HitResult Structure (by ref)"))
  (bind _slidingcharacter (`self.SlidingCharacter`))
  (`/Engine/EditorBlueprintResources/StandardMacros.IsValid` (`self.SlidingCharacter`)
    (:`Is Not Valid`
      (bind _asbp_platform_game_character (cast `/Game/PGTemplate/Blueprints/Characters/Core/BP_PlatformGameCharacter` OtherActor))
      (bind _output_get (set `self.SlidingCharacter` _asbp_platform_game_character))
      (set `self.StartingLocation` (`self.K2_GetActorLocation` _output_get))
      (`TimelineComponent.SetPlayRate` (`self.SlidePositionLerp`) (/ 1.0 (/ (- (`KismetMathLibrary.VSize` (`self.SlideEnd`)) (`KismetMathLibrary.VSize` (`KismetMathLibrary.InverseTransformLocation` (`self.GetTransform`) (`self.StartingLocation`)))) (`self.SlideSpeed`))))
      (set `/Game/PGTemplate/Blueprints/Characters/Core/BP_PlatformGameCharacter.CurrentSlide` self _output_get)
      (`self.K2_SetActorRotation` _output_get (`self.K2_GetActorRotation`) false)
      (`Character.PlayAnimMontage` _slidingcharacter "/Game/PGTemplate/Blueprints/Characters/Core/Animations/Mixamo/Movement/RunningSlide_UE_Montage.RunningSlide_UE_Montage" 1.0 "SlideStart")
      (set `/Game/PGTemplate/Blueprints/Characters/Core/BP_PlatformGameCharacter.ForceInputBlock` true _slidingcharacter)
      (set `/Game/PGTemplate/Blueprints/Characters/Core/BP_PlatformGameCharacter.isSliding` true _slidingcharacter)
      (`CharacterMovementComponent.SetMovementMode` (`Character.CharacterMovement` _slidingcharacter) "MOVE_Flying" 0)
      (bind (_direction _lerpalpha) (`Timeline|SlidePositionLerp` :!via `PlayFromStart` :!label _label)
        (:`Update`
          (`self.K2_SetActorLocationAndRotation` (`self.SlidingCharacter`) (`KismetMathLibrary.VLerp` (`self.StartingLocation`) (+ (`self.K2_GetActorLocation`) (`KismetMathLibrary.GreaterGreater_VectorRotator` (`self.SlideEnd`) (`self.K2_GetActorRotation`))) _lerpalpha) (`SceneComponent.K2_GetComponentRotation` (`self.PlayerDetection`)) false false))
        (:`Finished`
          (`self.StopCharacterSliding`))))))

(event `StopSliding`
  (`self.StopCharacterSliding`)
  (goto _label :!via `Stop`))

(fn `StopCharacterSliding`
  (bind _slidingcharacter (`self.SlidingCharacter`))
  (`Character.PlayAnimMontage` _slidingcharacter "/Game/PGTemplate/Blueprints/Characters/Core/Animations/Mixamo/Movement/RunningSlide_UE_Montage.RunningSlide_UE_Montage" 1.0 "SlideEnd")
  (set `/Game/PGTemplate/Blueprints/Characters/Core/BP_PlatformGameCharacter.ForceInputBlock` false _slidingcharacter)
  (set `/Game/PGTemplate/Blueprints/Characters/Core/BP_PlatformGameCharacter.isSliding` false _slidingcharacter)
  (`CharacterMovementComponent.SetMovementMode` (`Character.CharacterMovement` _slidingcharacter) "MOVE_Falling" 0)
  (set `self.SlidingCharacter` null))

(fn `UserConstructionScript`
  (bind (_slideend_x _slideend_y _slideend_z) (`KismetMathLibrary.BreakVector` (`self.SlideEnd`)))
  (bind _playerdetection (`self.PlayerDetection`))
  (bind _returnvalue (`SceneComponent.K2_GetComponentLocation` (`self.PlayerDetection`)))
  (bind _returnvalue_x (`KismetMathLibrary.BreakVector` (/ (`self.SlideEnd`) 2.0)))
  (bind _relativelocation_x (`KismetMathLibrary.BreakVector` (`SceneComponent.RelativeLocation` _playerdetection)))
  (set `self.SlideEnd` (`KismetMathLibrary.MakeVector` _slideend_x 0.0 _slideend_z))
  (`SceneComponent.K2_SetRelativeLocation` (`self.PlayerDetection`) (`KismetMathLibrary.MakeVector` _returnvalue_x) false false)
  (bind _outhit (`KismetSystemLibrary.LineTraceSingle` _returnvalue (- _returnvalue (0.0 0.0 10000000.0)) "TraceTypeQuery1"))
  (if true
    (bind (_returnvalue_x_2 _returnvalue_y _returnvalue_z) (`KismetMathLibrary.BreakVector` (`KismetMathLibrary.InverseTransformLocation` (`self.GetTransform`) (`.Location` (`GameplayStatics.BreakHitResult` _outhit)))))
    (`SceneComponent.K2_SetRelativeLocation` _playerdetection (`KismetMathLibrary.MakeVector` _relativelocation_x 0.0 _returnvalue_z) false false)
    (`SceneComponent.K2_SetRelativeRotation` (`self.PlayerDetection`) (`KismetMathLibrary.FindLookAtRotation` (0.0 0.0 0.0) (`self.SlideEnd`)) false false)
    (`SceneComponent.SetRelativeScale3D` (`self.PlayerDetection`) (`KismetMathLibrary.MakeVector` (* (`KismetMathLibrary.VSize` (`self.SlideEnd`)) 0.015) 1.0 0.1))
    (else
      (`KismetSystemLibrary.PrintString` "NO SURFACE FOUND TO SLIDE ON!"))))