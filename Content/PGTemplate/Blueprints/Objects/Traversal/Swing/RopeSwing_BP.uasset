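; Swinging rope traversal object that a falling player character grabs on overlap, subject to a cooldown.
; A self-restarting timeline pitches the hinge across the swing arc, scaled by a momentum that flips each pass, decays every tick and can be boosted.
; Attaching moves the rope end to the character and swaps the loose cable for stiff and excess cables; detaching restores it.
; Construction sizes cables and detection volume from the rope end point.
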(event `AttachPlayer`
  (bind _stiffcable (`self.StiffCable`))
  (bind (_returnvalue_x _returnvalue_y _returnvalue_z) (`KismetMathLibrary.BreakVector` (`KismetMathLibrary.InverseTransformLocation` (`SceneComponent.K2_GetComponentToWorld` (`self.SwingHinge`)) (`self.K2_GetActorLocation` (`self.HangingCharacter`)))))
  (bind _returnvalue (+ _returnvalue_z 110.0))
  (`SceneComponent.K2_SetRelativeRotation` :`self` (`self.PlayerConnectionPoint`))
  (`SceneComponent.K2_SetRelativeLocation` (`self.SwingEnd`) (`KismetMathLibrary.MakeVector` 0.0 0.0 _returnvalue) false false)
  (bind _output_get (set `CableComponent.CableLength` (* _returnvalue -0.5) _stiffcable))
  (set `CableComponent.CableLength` (- (`self.InitialRopeLength`) (* _output_get 2.0)) (`self.ExcessCable`))
  (`SceneComponent.SetVisibility` _stiffcable true true)
  (`SceneComponent.SetVisibility` (`self.ExcessCable`) true false)
  (`SceneComponent.SetVisibility` (`self.LooseCable`) false false))

(event `DetachPlayer`
  (`SceneComponent.SetVisibility` (`self.StiffCable`) false true)
  (`SceneComponent.K2_SetRelativeLocation` (`self.SwingEnd`) (`KismetMathLibrary.MakeVector` 0.0 0.0 (* (`self.InitialRopeLength`) -1.0)) false true)
  (`SceneComponent.SetVisibility` (`self.ExcessCable`) false false)
  (`SceneComponent.SetVisibility` (`self.LooseCable`) true false)
  (set `self.HangingCharacter` null))

(event `StartSwing`
  (params (StartTime :type "Float (double-precision)"))
  (bind _swingarc (`self.SwingArc`))
  (`|ExecutionSequence`
    (:`then_0`
      (bind (_direction _swingarccompletion) (`Timeline|SwingTimeline` :`NewTime` StartTime :!via `SetNewTime` :!label _label)
        (:`Update`
          (`SceneComponent.K2_SetRelativeRotation` (`self.SwingHinge`) (`KismetMathLibrary.MakeRotator` 0.0 (* (`KismetMathLibrary.Lerp` (* _swingarc -0.5) (* _swingarc 0.5) _swingarccompletion) (`self.Momentum`))) false false))
        (:`Finished`
          (bind _output_get (set `self.Momentum` (* (`self.Momentum`) -1.0)))
          (if (not (`KismetMathLibrary.NearlyEqual_FloatFloat` _output_get 0.0 0.01))
            (`self.StartSwing` 0.0)))))
    (:`then_1`
      (goto _label))))

(event `self.ReceiveTick`
  (params (DeltaSeconds :type "Float (single-precision)"))
  (bind _elapsedtime (`self.ElapsedTime`))
  ;[1 1 1] Cooldown
  (if (< _elapsedtime (`self.Cooldown`))
    (set `self.ElapsedTime` (+ DeltaSeconds _elapsedtime)))
  ;[1 1 1] Momentum Decay
  (set `self.Momentum` (* (- 1.0 (`self.MomentumDecay`)) (`self.Momentum`))))

(event `self.PlayerDetection.OnComponentBeginOverlap`
  (params (OverlappedComponent :type "PrimitiveComponent Object Reference") (OtherActor :type "Actor Object Reference") (OtherComp :type "PrimitiveComponent Object Reference") (OtherBodyIndex :type Integer) (bFromSweep :type Boolean) (SweepResult :type "HitResult Structure (by ref)"))
  (bind _swingarc (`self.SwingArc`))
  (bind (_relativerotation_roll _relativerotation_pitch) (`KismetMathLibrary.BreakRotator` (`SceneComponent.RelativeRotation` (`self.SwingHinge`))))
  (if (and (>= (`self.ElapsedTime`) (`self.Cooldown`)) (not (`KismetSystemLibrary.IsValid` (`self.HangingCharacter`))))
    (bind _asbp_player_character (cast `/Game/PGTemplate/Blueprints/Characters/Player/BP_PlayerCharacter` OtherActor))
    (bind _charactermovement (`Character.CharacterMovement` _asbp_player_character))
    (bind _returnvalue_x (`KismetMathLibrary.BreakVector` (`CharacterMovementComponent.GetLastUpdateVelocity` _charactermovement)))
    (set `self.TargetMomentum` (/ _returnvalue_x 500.0))
    (`self.StartSwing` (/ (+ _relativerotation_pitch (* _swingarc 0.5)) _swingarc))
    (if (`NavMovementComponent.IsFalling` _charactermovement)
      (bind _output_get (set `self.HangingCharacter` _asbp_player_character))
      (`self.AttachPlayer`)
      (`/Game/PGTemplate/Blueprints/Characters/Core/BP_PlatformGameCharacter.GrabRope` _output_get self)
      (set `self.ElapsedTime` 0.0))))

(event `AddMomentum`
  (params (AddedMomentum :type "Float (double-precision)"))
  (set `self.Momentum` (`KismetMathLibrary.FClamp` (* (+ 1.0 (`KismetMathLibrary.Abs` AddedMomentum)) (`self.Momentum`)) -1.0)))

(event `SwitchSides`
  (params (InputDirection :type "Float (double-precision)"))
  (`SceneComponent.K2_AddRelativeRotation` (`self.PlayerConnectionPoint`) (struct :`Yaw` 180.0) false false))

(fn `UserConstructionScript`
  (bind _playerdetection (`self.PlayerDetection`))
  (bind _initialropelength (`self.InitialRopeLength`))
  (bind (_ropeend_x _ropeend_y _ropeend_z) (`KismetMathLibrary.BreakVector` (`self.RopeEnd`)))
  (bind _returnvalue (* _initialropelength -1.0))
  ;[1 1 1] Clamp Rope End & Retrieve Z for Rope Length
  (bind _output_get (set `self.RopeEnd` (`KismetMathLibrary.MakeVector` 0.0 0.0 _ropeend_z)))
  (set `self.InitialRopeLength` (* (.z _output_get) -1.0))
  (set `CableComponent.CableLength` (* _initialropelength 0.5) (`self.LooseCable`))
  (`SceneComponent.K2_SetRelativeLocation` (`self.SwingEnd`) (`KismetMathLibrary.MakeVector` 0.0 0.0 _returnvalue) false false)
  (`SceneComponent.K2_SetRelativeLocationAndRotation` _playerdetection (`KismetMathLibrary.MakeVector` 0.0 0.0 (* _returnvalue 0.5)) (`KismetMathLibrary.MakeRotator` 0.0) false false)
  (`SceneComponent.SetRelativeScale3D` _playerdetection (`KismetMathLibrary.MakeVector` 0.05 0.05 (* (`self.InitialRopeLength`) 0.015)))
  (`SceneComponent.SetVisibility` (`self.StiffCable`) false true)
  (`SceneComponent.SetVisibility` (`self.ExcessCable`) false false))