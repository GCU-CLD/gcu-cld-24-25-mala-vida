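; Base platform-game character providing health, movement gaits, mantling, rope grabbing and object interaction, with a tintable mannequin material.
; Registered hits update a health widget, then trigger TakeHit, or drop carried objects, ragdoll and call Die.
; Mantling picks the nearest unblocked spot and drives montages through Motion Warping while input mappings are cleared.
; Interactive objects are highlighted by proximity, favoring carriables; collectibles enter an inventory and attach to facing-dependent hand sockets.
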(event `TakeHit`)

(event `Die`)

(event `RegisterHit`
  (params (ImpactVelocity :type "Vector Structure") (WorldHitLocation :type "Vector Structure") (DamageDone :type "Float (double-precision)"))
  (bind _currentlycarriedobject (`self.CurrentlyCarriedObject`))
  ;[1 0 0] Register Hit (may include damage)
  (bind _output_get (set `self.Health` (- (`self.Health`) DamageDone)))
  (`/Game/PGTemplate/Blueprints/Characters/Core/UI/HealthBar_W.UpdateHealth` (`self.HealthBarWidget`) _output_get 1.0)
  (if (<= _output_get 0.0)
    (if (== (`GameplayStatics.GetObjectClass` self) "/Game/PGTemplate/Blueprints/Characters/Player/BP_PlayerCharacter.BP_PlayerCharacter_C")
      (`self.BlockControl` false))
    (`/Engine/EditorBlueprintResources/StandardMacros.IsValid` _currentlycarriedobject
      (:`Is Valid`
        (`/Game/PGTemplate/Blueprints/Objects/Carried/Core/CarriedObject_IO.ForceDrop` _currentlycarriedobject))
      (:`Is Not Valid`
        _))
    (`self.Ragdoll`)
    (`PrimitiveComponent.AddImpulseAtLocation` (`self.Mesh`) ImpactVelocity WorldHitLocation "None")
    (`self.Die`)
    (else
      (`self.TakeHit`))))

(event `self.ReceiveBeginPlay`
  ;[0 1 0] BeginPlay Actions
  (set `self.GameModeREF` (cast `/Game/PGTemplate/Blueprints/Core/BP_PlatformGame_GameMode` (`GameplayStatics.GetGameMode`) :!pure true))
  (set `self.Health` 1.0)
  (set `self.HealthBarWidget` (cast `/Game/PGTemplate/Blueprints/Characters/Core/UI/HealthBar_W` (`WidgetComponent.GetWidget` (`self.Widget`)) :!pure true))
  (`self.UnBlockControl`))

(event `self.ReceiveTick`
  (params (DeltaSeconds :type "Float (single-precision)"))
  (bind _widget (`self.Widget`))
  ;[1 1 1] Keep Widget properly aligned
  (`SceneComponent.K2_SetWorldRotation` _widget (struct :`Yaw` 90.0) false false)
  (`SceneComponent.K2_SetWorldLocation` _widget (+ (`SceneComponent.GetSocketLocation` (`self.Mesh`) "pelvis") (0.0 0.0 100.0)) false false))

(event `Grab`
  (bind (_returnvalue_roll _returnvalue_pitch _returnvalue_yaw) (`KismetMathLibrary.BreakRotator` (`self.K2_GetActorRotation`)))
  (bind _returnvalue (`self.GetComponentByClass` (`self.CurrentInteractiveObject`) "/Script/Engine.StaticMeshComponent"))
  ;[0 0 0] Grabbing Objects
  (`SceneComponent.K2_AttachToComponent` _returnvalue (`self.Mesh`) (select `bool` (> (`KismetMathLibrary.Abs` _returnvalue_yaw) 90.0) :`false` "hand_l" :`true` "hand_r" :!type "Name") "SnapToTarget" "KeepWorld" "KeepWorld" true)
  (`SceneComponent.K2_AddRelativeLocation` _returnvalue (10.0 0.0 0.0) false false)
  (set `self.CurrentlyHeldMesh` _returnvalue))

(event `PutAway`
  ;[0 0 0] Grabbing Objects
  (`SceneComponent.SetVisibility` (`self.CurrentlyHeldMesh`) false false))

(event `Mantle`
  (params (isFalling :type Boolean) (`1mMantle` :type Boolean))
  (bind _nearestspot (`self.GetNearestMantleSpot`))
  (bind _charactermovement (`self.CharacterMovement`))
  (bind _playerentry (`/Game/PGTemplate/Blueprints/Objects/Traversal/MantleSpot_BP.PlayerEntry` (`self.CurrentMantleSpot`)))
  (bind _playerclimbposition (`/Game/PGTemplate/Blueprints/Objects/Traversal/MantleSpot_BP.PlayerClimbPosition` (`self.CurrentMantleSpot`)))
  (bind _playerexit (`/Game/PGTemplate/Blueprints/Objects/Traversal/MantleSpot_BP.PlayerExit` (`self.CurrentMantleSpot`)))
  (bind _returnvalue (`SceneComponent.K2_GetComponentLocation` (`/Game/PGTemplate/Blueprints/Objects/Traversal/MantleSpot_BP.HandAnchor` _nearestspot)))
  ;[0 0 0] Mantle System
  (`/Engine/EditorBlueprintResources/StandardMacros.IsValid` _nearestspot
    (:`Is Valid`
      (set `self.HandAnchorLeft` (- _returnvalue (0.0 40.0 0.0)))
      (set `self.HandAnchorRight` (+ _returnvalue (0.0 40.0 0.0)))
      (bind _output_get (set `self.CurrentMantleSpot` _nearestspot))
      (`/Game/PGTemplate/Blueprints/Objects/Traversal/MantleSpot_BP.LockPhysicsObjects` _output_get)
      (`MotionWarpingComponent.AddOrUpdateWarpTarget` (`self.MotionWarping`) (make `MotionWarpingTarget` "EntryPosition" (`SceneComponent.K2_GetComponentLocation` _playerentry) (`SceneComponent.K2_GetComponentRotation` _playerentry)))
      (`MotionWarpingComponent.AddOrUpdateWarpTarget` (`self.MotionWarping`) (make `MotionWarpingTarget` "ExitPosition" (`SceneComponent.K2_GetComponentLocation` _playerexit) (`SceneComponent.K2_GetComponentRotation` _playerexit) _playerexit))
      (`MotionWarpingComponent.AddOrUpdateWarpTarget` (`self.MotionWarping`) (make `MotionWarpingTarget` "Climb" (`SceneComponent.K2_GetComponentLocation` _playerclimbposition) (`SceneComponent.K2_GetComponentRotation` _playerclimbposition)))
      (`self.BlockControl` false)
      (`CharacterMovementComponent.SetMovementMode` (`self.CharacterMovement`) "MOVE_Flying" 0)
      (`|PlayMontage` (`self.Mesh`) (select `bool` isFalling :`false` (select `bool` `1mMantle` :`false` "/Game/PGTemplate/Blueprints/Characters/Core/Animations/ALS/2m_MantleFromStanding_Montage.2m_MantleFromStanding_Montage" :`true` "/Game/PGTemplate/Blueprints/Characters/Core/Animations/ALS/1m_MantleFromStanding_LH_Montage.1m_MantleFromStanding_LH_Montage" :!type "AnimMontage Object Reference") :`true` "/Game/PGTemplate/Blueprints/Characters/Core/Animations/ALS/MantleFromFalling_Montage.MantleFromFalling_Montage") 1.25
        (:`OnCompleted`
          (`self.UnBlockControl`)
          (`/Game/PGTemplate/Blueprints/Objects/Traversal/MantleSpot_BP.UnlockPhysicsObjects` (`self.CurrentMantleSpot`))
          (`CharacterMovementComponent.ClearAccumulatedForces` _charactermovement)
          (set `MovementComponent.Velocity` (0.0 0.0 0.0) _charactermovement)
          (`CharacterMovementComponent.SetMovementMode` _charactermovement "MOVE_Walking" 0))))))

(event `UpdateHealth`
  (params (NewHealthValue :type "Float (double-precision)") (HealthBarChangeSpeed :type "Float (double-precision)"))
  (`/Game/PGTemplate/Blueprints/Characters/Core/UI/HealthBar_W.UpdateHealth` (`self.HealthBarWidget`) NewHealthValue HealthBarChangeSpeed))

(event `SlideJump`
  (`/Game/PGTemplate/Blueprints/Objects/Traversal/Slide_BP.StopSliding` (`self.CurrentSlide`))
  (`self.LaunchCharacter` (`KismetMathLibrary.GreaterGreater_VectorRotator` (`self.SlideJumpForce`) (`self.K2_GetActorRotation`))))

(event `Footstep`
  (params (LeftFoot :type Boolean) (FootstepType :type "/Game/PGTemplate/Blueprints/Characters/Core/Animations/FootstepType Enum" :default "NewEnumerator0") (VolumeMultiplier :type "Float (double-precision)" :default 1.0))
  (`/Game/PGTemplate/Blueprints/Characters/Core/C_FootstepSystem.PlayFootstep` (`self.C_FootstepSystem`) LeftFoot FootstepType VolumeMultiplier))

(fn `AddNewInteractiveObject`
  (params (ObjectToAdd :type "/Game/PGTemplate/Blueprints/Objects/Core/InteractionObject_BP Object Reference (by ref)"))
  (`KismetArrayLibrary.Array_Add` (`self.InteractiveObjects`) ObjectToAdd)
  (set `self.NearestInteractiveObject` (`self.GetNearestInteractiveObject`)))

(fn `AddNewMantleSpot`
  (params (MantleSpot :type "/Game/PGTemplate/Blueprints/Objects/Traversal/MantleSpot_BP Object Reference (by ref)"))
  (`KismetArrayLibrary.Array_Add` (`self.MantleSpots`) MantleSpot))

(fn `AddToInventory`
  (params (ObjectToAdd :type "/Game/PGTemplate/Blueprints/Objects/Collectibles/Core/IO_CollectibleObject_BP Object Reference"))
  (`self.K2_AttachToActor` ObjectToAdd self "None" "KeepRelative" "KeepRelative" "KeepRelative" true)
  (`KismetArrayLibrary.Array_Add` (`self.Inventory`) ObjectToAdd)
  (`/Game/PGTemplate/Blueprints/Characters/Player/UI/PlayerHUD_W.Add to Inventory` (`/Game/PGTemplate/Blueprints/Core/BP_PlatformGame_GameMode.PlayerHUD` (`self.GameModeREF`)) (`/Game/PGTemplate/Blueprints/Objects/Collectibles/Core/IO_CollectibleObject_BP.ObjectName` ObjectToAdd)))

(fn `BlockControl`
  (params (WallJumping :type Boolean))
  (bind _returnvalue (pcsubsystem `EnhancedInputLocalPlayerSubsystem` (`GameplayStatics.GetPlayerController` 0)))
  (`MovementComponent.StopMovementImmediately` (`self.CharacterMovement`))
  (`EnhancedInputSubsystemInterface.ClearAllMappings` _returnvalue)
  (if WallJumping
    (`EnhancedInputSubsystemInterface.AddMappingContext` _returnvalue "/Game/PGTemplate/Blueprints/Characters/Player/Input/IMC_WallJumping.IMC_WallJumping" 0 (struct))
    (else
      (set `self.ForceInputBlock` true))))

(fn `CheckInventory`
  (params (CheckedObject :type "/Game/PGTemplate/Blueprints/Objects/Collectibles/Core/IO_CollectibleObject_BP Object Reference"))
  (returns (ObjectFound :type Boolean))
  (bind _returnvalue (`KismetArrayLibrary.Array_Find` (`self.Inventory`) CheckedObject))
  (`KismetSystemLibrary.PrintString` (`KismetStringLibrary.Conv_IntToString` _returnvalue))
  (return (> _returnvalue -1)))

(fn `FinishIncompleteTurn`)

(fn `GetCurrentGait`
  (returns (GaitBySpeed :type "/Game/PGTemplate/Blueprints/Core/MovementGaits Enum") (GaitByPreference :type "/Game/PGTemplate/Blueprints/Core/MovementGaits Enum"))
  (bind _desiredmovementgait (`self.DesiredMovementGait`))
  (bind _gaitmovespeeds (`self.GaitMoveSpeeds`))
  (bind _returnvalue (`KismetMathLibrary.VSizeXY` (`CharacterMovementComponent.GetLastUpdateVelocity` (`self.CharacterMovement`))))
  (if (> _returnvalue (`BlueprintMapLibrary.Map_Find` _gaitmovespeeds "NewEnumerator0"))
    (if (> _returnvalue (`BlueprintMapLibrary.Map_Find` _gaitmovespeeds "NewEnumerator1"))
      (if (> _returnvalue (`BlueprintMapLibrary.Map_Find` _gaitmovespeeds "NewEnumerator2"))
        (return "NewEnumerator3" _desiredmovementgait)
        (else
          (return "NewEnumerator2" _desiredmovementgait)))
      (else
        (return "NewEnumerator1" _desiredmovementgait)))
    (else
      (return "NewEnumerator0" (`self.DesiredMovementGait`)))))

(fn `GetNearestInteractiveObject`
  (returns (NearestObject :type "/Game/PGTemplate/Blueprints/Objects/Core/InteractionObject_BP Object Reference"))
  (locals (CurrentNearestObject :type "/Game/PGTemplate/Blueprints/Objects/Core/InteractionObject_BP Object Reference") (CurrentShortestDistance :type "Float (double-precision)") (FoundCarriedObject :type Boolean))
  (bind _currentnearestobject (`local.CurrentNearestObject`))
  (bind _nearestinteractiveobject (`self.NearestInteractiveObject`))
  (set `local.CurrentShortestDistance` 9999999999999.0)
  (set `local.FoundCarriedObject` false)
  (for _array_element (`self.InteractiveObjects`)
    (bind _ascarried_object_io (cast `/Game/PGTemplate/Blueprints/Objects/Carried/Core/CarriedObject_IO` _array_element)
      (:`then`
        (if (not (== (`self.CurrentlyCarriedObject`) _ascarried_object_io))
          (set `local.FoundCarriedObject` true)
          (bind _returnvalue (`KismetMathLibrary.Vector_Distance` (`self.K2_GetActorLocation`) (`self.K2_GetActorLocation` _array_element)))
          (set `local.CurrentShortestDistance` _returnvalue :!label _label)
          (set `local.CurrentNearestObject` _array_element)))
      (:`CastFailed`
        (if (`local.FoundCarriedObject`)
          _
          (elif (< _returnvalue (`local.CurrentShortestDistance`))
            (goto _label))))))
  (`/Engine/EditorBlueprintResources/StandardMacros.IsValid` _nearestinteractiveobject
    (:`Is Valid`
      (`/Game/PGTemplate/Blueprints/Objects/Core/InteractionObject_BP.DeHighlight` _nearestinteractiveobject self))
    (:`Is Not Valid`
      _))
  (`/Engine/EditorBlueprintResources/StandardMacros.IsValid` _currentnearestobject
    (:`Is Valid`
      (`/Game/PGTemplate/Blueprints/Objects/Core/InteractionObject_BP.Highlight` _currentnearestobject self (`KismetMathLibrary.MakeColor` 0.715 0.0 0.5))
      (return _currentnearestobject))))

(fn `GetNearestMantleSpot`
  (returns (NearestSpot :type "/Game/PGTemplate/Blueprints/Objects/Traversal/MantleSpot_BP Object Reference") (`1mMantle` :type Boolean))
  (locals (LocalNearestSpot :type "/Game/PGTemplate/Blueprints/Objects/Traversal/MantleSpot_BP Object Reference") (Distance :type "Float (double-precision)" :default 99999999999999.0))
  (`/Engine/EditorBlueprintResources/StandardMacros.IsValid` (`self.CurrentlyCarriedObject`)
    (:`Is Valid`
      (return null false))
    (:`Is Not Valid`
      (for _array_element (`self.MantleSpots`)
        (bind _returnvalue (`KismetMathLibrary.Vector_Distance` (`self.K2_GetActorLocation`) (`SceneComponent.K2_GetComponentLocation` (`/Game/PGTemplate/Blueprints/Objects/Traversal/MantleSpot_BP.PlayerEntry` _array_element))))
        (if (and (> (`KismetMathLibrary.Dot_VectorVector` (`self.GetActorForwardVector` _array_element) (`self.GetActorForwardVector`)) 0.0) (< _returnvalue (`local.Distance`)) (not (`/Game/PGTemplate/Blueprints/Objects/Traversal/MantleSpot_BP.ExitBlocked` _array_element)))
          (set `local.LocalNearestSpot` _array_element)
          (set `local.Distance` _returnvalue)))
      (bind _localnearestspot (`local.LocalNearestSpot`)
        (:`then`
          (bind (_returnvalue_x _returnvalue_y _returnvalue_z) (`KismetMathLibrary.BreakVector` (- (`SceneComponent.K2_GetComponentLocation` (`/Game/PGTemplate/Blueprints/Objects/Traversal/MantleSpot_BP.PlayerExit` _localnearestspot)) (`self.K2_GetActorLocation`))))
          (return _localnearestspot (< _returnvalue_z 110.0)))
        (:`else`
          (return _localnearestspot false))))))

(fn `GrabRope`
  (params (RopeSwing :type "/Game/PGTemplate/Blueprints/Objects/Traversal/Swing/RopeSwing_BP Object Reference"))
  (bind (_returnvalue_roll _returnvalue_pitch _returnvalue_yaw) (`KismetMathLibrary.BreakRotator` (`self.K2_GetActorRotation`)))
  (bind (_returnvalue_x _returnvalue_y _returnvalue_z) (`KismetMathLibrary.BreakVector` (`self.K2_GetActorLocation`)))
  (bind (_returnvalue_roll_2 _returnvalue_pitch_2 _returnvalue_yaw_2) (`KismetMathLibrary.BreakRotator` (`self.K2_GetActorRotation`)))
  (bind _charactermovement (`self.CharacterMovement`))
  (bind (_returnvalue_x_2 _returnvalue_y_2) (`KismetMathLibrary.BreakVector` (`SceneComponent.K2_GetComponentLocation` (`/Game/PGTemplate/Blueprints/Objects/Traversal/Swing/RopeSwing_BP.SwingEnd` (`local.RopeSwing`)))))
  (set `self.isOnRope` true)
  (set `self.CurrentRope` RopeSwing)
  (`self.K2_SetActorRotation` (`KismetMathLibrary.MakeRotator` 0.0 0.0 (`KismetMathLibrary.SelectFloat` 0.0 180.0 (or (< _returnvalue_yaw 90.0) (> _returnvalue_yaw 270.0)))))
  (`self.PlayAnimMontage` "/Game/PGTemplate/Blueprints/Objects/Traversal/Swing/Animation/Hanging_Montage.Hanging_Montage")
  ;[1 1 1] Position Player on Rope
  (`self.K2_SetActorLocation` (`KismetMathLibrary.MakeVector` (+ _returnvalue_x_2 (`KismetMathLibrary.SelectFloat` 6.0 -6.0 (> _returnvalue_yaw_2 0.0))) _returnvalue_y_2 _returnvalue_z))
  ;[1 1 1] Attach Actor to Rope End
  (`MovementComponent.StopMovementImmediately` _charactermovement)
  (`CharacterMovementComponent.SetMovementMode` _charactermovement "MOVE_Flying" 0)
  (`self.K2_AttachToComponent` (`/Game/PGTemplate/Blueprints/Objects/Traversal/Swing/RopeSwing_BP.PlayerConnectionPoint` (`local.RopeSwing`)) "None" "KeepWorld" "KeepWorld" "KeepRelative"))

(fn `isFacingRight`
  (returns (isFacingRight :type Boolean))
  (bind (_returnvalue_roll _returnvalue_pitch _returnvalue_yaw) (`KismetMathLibrary.BreakRotator` (`self.K2_GetActorRotation`)))
  (return (not (or (< _returnvalue_yaw -90.0) (> _returnvalue_yaw 90.0)))))

(fn `LineTraceToFloorPlusCapsuleHalfHeight`
  (params (StartPoint :type "Vector Structure")))

(fn `PlayLoopingSoundFromAnim`
  (params (SoundToPlay :type "SoundBase Object Reference") (SoundName :type Name))
  (bind _returnvalue (`GameplayStatics.SpawnSoundAttached` SoundToPlay (`self.Mesh`) "None" (0.0 0.0 0.0) (struct) "KeepRelativeOffset" false 1.0 1.0 0.0 null null))
  (`BlueprintMapLibrary.Map_Add` (`self.LoopingSoundsFromAnim`) SoundName _returnvalue)
  (`AudioComponent.Play` _returnvalue 0.0))

(fn `Ragdoll`
  (bind _mesh (`self.Mesh`))
  (`self.StopAnimMontage` (`self.GetCurrentMontage`))
  (`PrimitiveComponent.SetCollisionEnabled` (`self.CapsuleComponent`) "NoCollision")
  (`PrimitiveComponent.SetCollisionEnabled` _mesh "QueryAndPhysics")
  (`CharacterMovementComponent.ClearAccumulatedForces` (`self.CharacterMovement`))
  (`PrimitiveComponent.SetSimulatePhysics` _mesh true))

(fn `RemoveInteractiveObject`
  (params (Item :type "/Game/PGTemplate/Blueprints/Objects/Core/InteractionObject_BP Object Reference (by ref)"))
  (`KismetArrayLibrary.Array_RemoveItem` (`self.InteractiveObjects`) Item)
  (set `self.NearestInteractiveObject` (`self.GetNearestInteractiveObject`)))

(fn `RemoveMantleSpot`
  (params (MantleSpot :type "/Game/PGTemplate/Blueprints/Objects/Traversal/MantleSpot_BP Object Reference (by ref)"))
  (`KismetArrayLibrary.Array_RemoveItem` (`self.MantleSpots`) MantleSpot))

(fn `RetrieveFromInventory`
  (params (ObjectToRetrieve :type "/Game/PGTemplate/Blueprints/Objects/Collectibles/Core/IO_CollectibleObject_BP Object Reference"))
  (bind (_returnvalue_roll _returnvalue_pitch _returnvalue_yaw) (`KismetMathLibrary.BreakRotator` (`self.K2_GetActorRotation`)))
  (bind _collectiblemesh (`/Game/PGTemplate/Blueprints/Objects/Collectibles/Core/IO_CollectibleObject_BP.CollectibleMesh` ObjectToRetrieve))
  (bind _output_get (set `self.CurrentlyHeldMesh` _collectiblemesh))
  (`SceneComponent.SetVisibility` _output_get true false)
  (`SceneComponent.K2_AttachToComponent` _collectiblemesh (`self.Mesh`) (select `bool` (> (`KismetMathLibrary.Abs` _returnvalue_yaw) 90.0) :`false` "hand_l" :`true` "hand_r" :!type "Name") "KeepRelative" "KeepRelative" "KeepRelative" true)
  (`SceneComponent.K2_SetRelativeLocationAndRotation` :`self` _collectiblemesh))

(fn `RoundToDecimals`
  (params (Float :type "Float (double-precision)") (Decimals :type Integer))
  (returns (RoundedFloat :type "Float (double-precision)"))
  (bind _returnvalue (`KismetMathLibrary.MultiplyMultiply_FloatFloat` 10.0 (`KismetMathLibrary.Conv_IntToDouble` Decimals)))
  (return (/ (`KismetMathLibrary.Conv_IntToDouble` (`KismetMathLibrary.Round` (* Float _returnvalue))) _returnvalue)))

(fn `SetCapsuleCollision`
  (`PrimitiveComponent.SetCollisionEnabled` (`self.CapsuleComponent`) "NoCollision"))

(fn `SetDesiredMovementGait`
  (params (NewGait :type "/Game/PGTemplate/Blueprints/Core/MovementGaits Enum" :default "NewEnumerator0"))
  (bind (_value _returnvalue) (`BlueprintMapLibrary.Map_Find` (`self.AcceptableMoveGaits`) (`local.NewGait`)))
  (if (not (`KismetSystemLibrary.IsValid` (`self.CurrentlyCarriedObject`)))
    (if (and (`|EnumInequality` NewGait (`.GaitByPreference` (`self.GetCurrentGait`))) _value _returnvalue)
      (set `CharacterMovementComponent.MaxWalkSpeed` (`BlueprintMapLibrary.Map_Find` (`self.GaitMoveSpeeds`) NewGait) (`self.CharacterMovement`))
      (set `self.DesiredMovementGait` NewGait))))

(fn `SetHands`
  (params (HandPose :type "/Game/PGTemplate/Blueprints/Core/Hands Enum" :default "NewEnumerator0"))
  (set `self.HandState` HandPose))

(fn `StopLoopingSoundFromAnim`
  (params (SoundName :type Name))
  (`AudioComponent.Stop` (`BlueprintMapLibrary.Map_Find` (`self.LoopingSoundsFromAnim`) SoundName)))

(fn `StopRagdolling`
  (bind _mesh (`self.Mesh`))
  (bind _mesh_2 (`self.Mesh`))
  (`SkeletalMeshComponent.ResetAllBodiesSimulatePhysics` (`self.Mesh`))
  (`PrimitiveComponent.SetCollisionEnabled` (`self.CapsuleComponent`) "QueryAndPhysics")
  (`PrimitiveComponent.SetSimulatePhysics` _mesh_2 false)
  (`PrimitiveComponent.SetCollisionEnabled` _mesh_2 "QueryOnly")
  (`CharacterMovementComponent.ClearAccumulatedForces` (`self.CharacterMovement`))
  (`SceneComponent.K2_SetWorldLocation` _mesh (+ (`SceneComponent.K2_GetComponentLocation` (`self.CapsuleComponent`)) (0.0 0.0 -90.0)) false false)
  (`SceneComponent.K2_SetRelativeRotation` _mesh (struct :`Yaw` 270.0) false false))

(fn `UnBlockControl`
  (message `EnhancedInputSubsystemInterface.AddMappingContext` (pcsubsystem `EnhancedInputLocalPlayerSubsystem` (`GameplayStatics.GetPlayerController` 0)) "/Game/PGTemplate/Blueprints/Characters/Player/Input/IMC_Default.IMC_Default" 0 (struct))
  (set `self.ForceInputBlock` false))

(fn `UserConstructionScript`
  (bind _mesh (`self.Mesh`))
  (`|ExecutionSequence`
    (:`then_0`
      (`SceneComponent.K2_AttachToComponent` (`self.RightHand`) _mesh "hand_r" "SnapToTarget" "KeepRelative" "SnapToTarget" true)
      (`SceneComponent.K2_AttachToComponent` (`self.LeftHand`) _mesh "hand_l" "SnapToTarget" "SnapToTarget" "SnapToTarget" true)
      (`SceneComponent.K2_AttachToComponent` (`self.CratePosition`) _mesh "hand_r" "KeepWorld" "KeepWorld" "KeepRelative" true))
    (:`then_1`
      (bind _returnvalue (`KismetMaterialLibrary.CreateDynamicMaterialInstance` "/Game/PGTemplate/Blueprints/Characters/Core/Materials/M_UEFN_Mannequin.M_UEFN_Mannequin"))
      (`MaterialInstanceDynamic.SetVectorParameterValue` _returnvalue "HeadColour" (`self.HeadColor`))
      (`MaterialInstanceDynamic.SetVectorParameterValue` _returnvalue "HandsColour" (`self.HandsColour`))
      (`MaterialInstanceDynamic.SetVectorParameterValue` _returnvalue "ShirtColor" (`self.ShirtColour`))
      (`MaterialInstanceDynamic.SetVectorParameterValue` _returnvalue "UpperArmColour" (`self.UpperArmsColour`))
      (`MaterialInstanceDynamic.SetVectorParameterValue` _returnvalue "LowerArmColour" (`self.LowerArmsColour`))
      (`MaterialInstanceDynamic.SetVectorParameterValue` _returnvalue "UpperLegColour" (`self.UpperLegColour`))
      (`MaterialInstanceDynamic.SetVectorParameterValue` _returnvalue "LowerLegColour" (`self.LowerLegColour`))
      (`MaterialInstanceDynamic.SetVectorParameterValue` _returnvalue "FeetColour" (`self.FeetColour`))
      (`MaterialInstanceDynamic.SetVectorParameterValue` _returnvalue "WaistColour" (`self.WaistColour`))
      (`PrimitiveComponent.SetMaterial` (`self.Mesh`) 0 _returnvalue))))